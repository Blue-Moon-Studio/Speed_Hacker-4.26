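; BP_Item is an item actor whose mesh and data come from an entry in an ItemDataAssetMaster data asset.
; The construction script loads the Items asset through CreateAssetData and GetAsset, looks up the Item entry, then sets ItemMesh and caches ItemStruct.
; BeginPlay repeats the lookup to refresh ItemStruct.
; The actor has no active overlap, tick or pickup logic.
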(event EventBeginPlay
  (bind _asitem_data_asset_master (Utilities|Casting|CastToItemDataAssetMaster (Class|AssetRegistryHelpers|GetAsset (Class|AssetRegistryHelpers|CreateAssetData "/Game/Inventory/Items.Items" false))))
  (Variables|Default|SetItemStruct (Utilities|Array|Get(acopy) (Variables|/Game/Inventory/NEPASTOUCHER/ItemDataAssetMaster.ItemDataAssetMaster_C|GetItems _asitem_data_asset_master) (Variables|Default|GetItem))))

(event Collision|EventActorBeginOverlap
  (params (OtherActor :type Actor%20Object%20Reference)))

(event EventTick
  (params (DeltaSeconds :type Float%20%28single-precision%29)))

(fn ConstructionScript
  (bind _asitem_data_asset_master (Utilities|Casting|CastToItemDataAssetMaster (Class|AssetRegistryHelpers|GetAsset (Class|AssetRegistryHelpers|CreateAssetData "/Game/Inventory/Items.Items" false))))
  (Components|StaticMesh|SetStaticMesh (Variables|Default|GetItemMesh) (.StaticMesh (Utilities|Struct|BreakS_Item (Utilities|Array|Get(acopy) (Variables|/Game/Inventory/NEPASTOUCHER/ItemDataAssetMaster.ItemDataAssetMaster_C|GetItems _asitem_data_asset_master) (Variables|Default|GetItem)))))
  (Variables|Default|SetItemStruct (Utilities|Array|Get(acopy) (Variables|/Game/Inventory/NEPASTOUCHER/ItemDataAssetMaster.ItemDataAssetMaster_C|GetItems _asitem_data_asset_master) (Variables|Default|GetItem))))